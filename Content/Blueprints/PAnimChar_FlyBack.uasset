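; PAnimChar_FlyBack is a character Blueprint that plays a fly-back animation and turns into a ragdoll after hitting a wall.
; On BeginPlay, bodies below the pelvis simulate under a strong Physical Animation profile.
; StartFlyBack enables root motion from everything and sets the AnimBP's ShouldFly flag.
; The first mesh hit on a "Wall"-tagged component, after a short delay, simulates the pelvis too, enables gravity and switches to the Ragdoll profile.
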(event `self.ReceiveBeginPlay`
  (`SkeletalMeshComponent.SetAllBodiesBelowSimulatePhysics` (`self.Mesh`) (`KismetStringLibrary.Conv_StringToName` "pelvis") true false)
  (`PhysicalAnimationComponent.SetSkeletalMeshComponent` (`self.PhysicalAnimation`) (`self.Mesh`))
  (`PhysicalAnimationComponent.ApplyPhysicalAnimationProfileBelow` (`self.PhysicalAnimation`) "pelvis" "FullBodyStrong" true false))

(event `self.Mesh.OnComponentHit`
  (params (HitComponent :type "PrimitiveComponent Object Reference") (OtherActor :type "Actor Object Reference") (OtherComp :type "PrimitiveComponent Object Reference") (NormalImpulse :type "Vector Structure") (Hit :type "HitResult Structure (by ref)"))
  (bind _mesh (`self.Mesh`))
  (if (and (`ActorComponent.ComponentHasTag` OtherComp "Wall") (not (`self.HasRagdolled`)))
    (`KismetSystemLibrary.Delay` 0.2)
    ;[1 1 1] 开启Ragdoll并使根组件模拟物理
    (`SkeletalMeshComponent.SetAllBodiesBelowSimulatePhysics` _mesh (`KismetStringLibrary.Conv_StringToName` "pelvis") true true)
    (`PrimitiveComponent.SetEnableGravity` _mesh true)
    (`PhysicalAnimationComponent.ApplyPhysicalAnimationProfileBelow` (`self.PhysicalAnimation`) "pelvis" "Ragdoll" true false)
    (set `self.HasRagdolled` true)))

(event `StartFlyBack`
  (bind _returnvalue (`SkeletalMeshComponent.GetAnimInstance` (`self.Mesh`)))
  ;[1 1 1] 开始播放倒飞动画
  (`AnimInstance.SetRootMotionMode` _returnvalue "RootMotionFromEverything")
  (bind _asanim_bp_fly_back (cast `/Game/Blueprints/AnimBP/AnimBP_FlyBack` _returnvalue))
  (set `/Game/Blueprints/AnimBP/AnimBP_FlyBack.ShouldFly` true _asanim_bp_fly_back))

(fn `UserConstructionScript`)